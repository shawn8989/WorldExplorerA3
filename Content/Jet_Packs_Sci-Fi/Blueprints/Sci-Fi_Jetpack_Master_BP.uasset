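; Master jetpack actor for a character, swapping mesh, anim Blueprint, exhaust particles and engine audio by jetpack type.
; Receives type, equip, flying and movement input messages, forwarding state to the jetpack anim instance.
; UpdateType, also run at construction, rebuilds effects on name-matched sockets and creates dynamic materials.
; Flight state and input drive particle scale, smoothed audio volume and pitch, engine heat and Grav glow, while Winged packs fade wings on equip.
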(event `Update Parent`
  (bind _ascharacter (cast `Character` (`self.GetParentActor`) :!label _label))
  (set `self.Parent` _ascharacter))

(event `self.ReceiveBeginPlay`
  (goto _label))

(event `/Game/Jet_Packs_Sci-Fi/Blueprints/Sci-Fi_Jetpack_Inputs_BPI.Sci Jetpack Type`
  (params (Type :type "/Game/Jet_Packs_Sci-Fi/Blueprints/Sci-Fi__Jetpacks_Enum Enum" :default "NewEnumerator0"))
  ;[1 1 1] Jetpack Inputs
  ; Added By the Jetpack Inputs BPI
  ;
  ; Allows the jetpack actor to know what state it should be in. Also includes some changes made based on those. Equipping will enable the equipping value, on a timer based on the current jetpack type.
  (set `self.Current Jetpack Type` Type)
  (`self.Update Type`))

(event `/Game/Jet_Packs_Sci-Fi/Blueprints/Sci-Fi_Jetpack_Inputs_BPI.Sci Jetpack Flying`
  (params (True :type Boolean))
  (bind _jetpack_anim_instance (`self.Jetpack Anim Instance`))
  ;[1 1 1] Jetpack Inputs
  ; Added By the Jetpack Inputs BPI
  ;
  ; Allows the jetpack actor to know what state it should be in. Also includes some changes made based on those. Equipping will enable the equipping value, on a timer based on the current jetpack type.
  (bind _output_get (set `self.Jetpack_Flying` True))
  (`/Engine/EditorBlueprintResources/StandardMacros.IsValid` _jetpack_anim_instance
    (:`Is Valid`
      (message `/Game/Jet_Packs_Sci-Fi/Blueprints/Sci-Fi_Jetpack_Inputs_BPI.Sci Jetpack Flying` _jetpack_anim_instance _output_get))
    (:`Is Not Valid`
      _))
  (if (`self.Jetpack_Flying`)
    ;;[1 1 1] Exhaust particles use "Scale" as a spawn rate scaling parameter.
    ;; 0 disables particles, 1 is default.
    (bind (_direction _scale) (`Timeline|Particle Scale` :!label _label_2)
      (:`Update`
        (for _array_element (`self.Particles`)
          (`/Engine/EditorBlueprintResources/StandardMacros.IsValid` _array_element
            (:`Is Valid`
              (`ParticleSystemComponent.SetFloatParameter` _array_element "Scale" _scale))))
        (if (`|EnumEquality` (`self.Current Jetpack Type`) "NewEnumerator2")
          (`MaterialInstanceDynamic.SetScalarParameterValue` (`self.Grav_MI`) "EMIS Power" (`KismetMathLibrary.Lerp` 0.0 0.55 _scale)))))
    (else
      (goto _label_2 :!via `Reverse`))))

(event `/Game/Jet_Packs_Sci-Fi/Blueprints/Sci-Fi_Jetpack_Inputs_BPI.Sci Jetpack Inputs`
  (params (Forward :type "Float (single-precision)") (`Move Right` :type "Float (single-precision)") (`Turn Right` :type "Float (single-precision)") (`Move Up` :type "Float (single-precision)"))
  (bind _jetpack_anim_instance (`self.Jetpack Anim Instance`))
  (bind _jetpack_flying (`self.Jetpack_Flying`))
  (bind _returnvalue (+ (`KismetMathLibrary.Abs` (`self.Forward`)) (`KismetMathLibrary.Abs` (`self.Right`)) (* (`KismetMathLibrary.Abs` (`self.Turn_Right`)) 0.35) (* (`self.Up`) 1.2)))
  ;[1 1 1] Jetpack Inputs
  ; Added By the Jetpack Inputs BPI
  ;
  ; Allows the jetpack actor to know what state it should be in. Also includes some changes made based on those. Equipping will enable the equipping value, on a timer based on the current jetpack type.
  (bind _output_get (set `self.Forward` Forward))
  (bind _output_get_2 (set `self.Right` `Move Right`))
  (bind _output_get_3 (set `self.Turn_Right` `Turn Right`))
  (bind _output_get_4 (set `self.Up` `Move Up`))
  (`/Engine/EditorBlueprintResources/StandardMacros.IsValid` _jetpack_anim_instance
    (:`Is Valid`
      (message `/Game/Jet_Packs_Sci-Fi/Blueprints/Sci-Fi_Jetpack_Inputs_BPI.Sci Jetpack Inputs` _jetpack_anim_instance _output_get _output_get_2 _output_get_3 _output_get_4))
    (:`Is Not Valid`
      _))
  (`self.Update Audio Multiplier`)
  (if (`|EnumEquality` (`self.Current Jetpack Type`) "NewEnumerator2")
    ;;[1 1 1] Adjust material to reflect power for anti grav jetpacks glowing core
    (`MaterialInstanceDynamic.SetScalarParameterValue` (`self.Grav_MI`) "EMIS Power" (* (`KismetMathLibrary.MapRangeClamped` _returnvalue -1.2 3.55 0.45 4.0) (`KismetMathLibrary.Conv_BoolToDouble` _jetpack_flying))))
  ;;[1 1 1] Adjust heat level or glow for engines
  (bind _output_get_5 (set `self.Jetpack Heat Level` (`KismetMathLibrary.FInterpTo` (`self.Jetpack Heat Level`) (* (`KismetMathLibrary.MapRangeClamped` _returnvalue -1.2 3.55 0.18 1.0) (`KismetMathLibrary.Conv_BoolToDouble` _jetpack_flying) (`self.Heat Glow Multiplier`)) (`GameplayStatics.GetWorldDeltaSeconds`) (`self.Heat Glow Change Speed`))))
  (`MaterialInstanceDynamic.SetScalarParameterValue` (`self.Jetpack_MI`) "EMIS Power" _output_get_5))

(event `/Game/Jet_Packs_Sci-Fi/Blueprints/Sci-Fi_Jetpack_Inputs_BPI.Sci Jetpack Equip`
  (params (Equip :type Boolean))
  (bind _jetpack_anim_instance (`self.Jetpack Anim Instance`))
  ;[1 1 1] Jetpack Inputs
  ; Added By the Jetpack Inputs BPI
  ;
  ; Allows the jetpack actor to know what state it should be in. Also includes some changes made based on those. Equipping will enable the equipping value, on a timer based on the current jetpack type.
  (`|ExecutionSequence`
    (:`then_0`
      (if Equip
        (set `self.Equipping` true)
        (set `self.Using Jetpack` true)
        (else
          (set `self.Unequiping` true)))
      (switch `/Game/Jet_Packs_Sci-Fi/Blueprints/Sci-Fi__Jetpacks_Enum` (`self.Current Jetpack Type`)
        (:`NewEnumerator0`
          (`KismetSystemLibrary.K2_SetTimerDelegate` (delegate `Un/Equip Over`) 0.1 :!label _label_3))
        (:`NewEnumerator1`
          (goto _label_3))
        (:`NewEnumerator2`
          (goto _label_3))
        (:`NewEnumerator4`
          (goto _label_3))
        (:`NewEnumerator3`
          (goto _label_3))
        (:`NewEnumerator5`
          (goto _label_3))
        (:`NewEnumerator6`
          (`|ExecutionSequence`
            (:`then_0`
              (goto _label_3))
            (:`then_1`
              (if (`self.Equipping`)
                ;;[1 1 1] Adjust wings opacity for winged jetpack upon turning on/off
                (bind (_direction _lerp) (`Timeline|Winged Fade Timeline` :!label _label_4)
                  (:`Update`
                    (`MaterialInstanceDynamic.SetScalarParameterValue` (`self.Wings_MI`) "Opacity" _lerp)))
                (else
                  (goto _label_4 :!via `Reverse`))))))))
    (:`then_1`
      (`/Engine/EditorBlueprintResources/StandardMacros.IsValid` _jetpack_anim_instance
        (:`Is Valid`
          (message `/Game/Jet_Packs_Sci-Fi/Blueprints/Sci-Fi_Jetpack_Inputs_BPI.Sci Jetpack Equip` _jetpack_anim_instance Equip))))))

(event `Un/Equip Over`
  ;[1 1 1] Jetpack Inputs
  ; Added By the Jetpack Inputs BPI
  ;
  ; Allows the jetpack actor to know what state it should be in. Also includes some changes made based on those. Equipping will enable the equipping value, on a timer based on the current jetpack type.
  (`|ExecutionSequence`
    (:`then_0`
      (if (not (`self.Equipping`))
        (set `self.Using Jetpack` false)))
    (:`then_1`
      (set `self.Equipping` false)
      (set `self.Unequiping` false))))

(event `Update Type`
  (bind _current_jetpack_type (`self.Current Jetpack Type`))
  (bind _jetpack (`self.Jetpack`))
  (bind _jetpack_2 (`self.Jetpack`))
  (bind _current_jetpack_type_2 (`self.Current Jetpack Type`))
  (bind _jetpack_3 (`self.Jetpack`))
  (bind _jetpack_4 (`self.Jetpack`))
  (bind _jetpack_5 (`self.Jetpack`))
  (bind _sounds (`self.Sounds`))
  (bind _item (`KismetArrayLibrary.Array_Get` (`self.Jetpack Meshes`) (`KismetMathLibrary.Conv_ByteToInt` (`self.Current Jetpack Type`))))
  ;[1 1 1] Update the type of jetpack/meshes used, and set up the required values/mesh location for it.
  ;;[1 1 1] Clear old particles, update jetpack to new mesh, and if handheld adjust its pose to match parent
  (`self.Clear Particles`)
  (`SkinnedMeshComponent.SetSkinnedAssetAndUpdate` _jetpack _item true)
  (for (_array_element _array_index) (`SkeletalMesh.Materials` _item)
    (`PrimitiveComponent.SetMaterial` _jetpack _array_index (break `SkeletalMaterial` _array_element))
    ;;[1 1 1] Confirm animation mode, mesh location, and parent fo rall non HandHeld packs
    (`SkeletalMeshComponent.SetAnimationMode` _jetpack_5 "AnimationBlueprint")
    (`SkinnedMeshComponent.SetLeaderPoseComponent` _jetpack_5 null)
    (`SceneComponent.K2_AttachToComponent` _jetpack_4 (`self.DefaultSceneRoot`) "spine_03" "SnapToTarget" "SnapToTarget" "SnapToTarget" true)
    (`SceneComponent.K2_SetRelativeLocationAndRotation` _jetpack_4 (`self.Jetpacks Relative Location Offset`) (struct) false true)
    (`|ExecutionSequence`
      (:`then_0`
        ;;[1 1 1] Set up animation blueprint and default values for Twin Fan packs
        (`SkeletalMeshComponent.SetAnimInstanceClass` _jetpack_2 (`KismetArrayLibrary.Array_Get` (`self.Jetpack Anim BPs`) (`KismetMathLibrary.Conv_ByteToInt` (`self.Current Jetpack Type`))))
        (bind _output_get (set `self.Jetpack Anim Instance` (`SkeletalMeshComponent.GetAnimInstance` _jetpack_2)))
        (`/Engine/EditorBlueprintResources/StandardMacros.IsValid` _output_get
          (:`Is Valid`
            (message `/Game/Jet_Packs_Sci-Fi/Blueprints/Sci-Fi_Jetpack_Inputs_BPI.Sci Jetpack Equip` _output_get (or (`self.Using Jetpack`) (`self.Equipping`)))
            (message `/Game/Jet_Packs_Sci-Fi/Blueprints/Sci-Fi_Jetpack_Inputs_BPI.Sci Jetpack Flying` _output_get (`self.Jetpack_Flying`)))
          (:`Is Not Valid`
            _))
        ;;[1 1 1] Spawn exhausts
        (`self.Clear Particles` :!label _label_5)
        (for _array_element_2 (`SceneComponent.GetAllSocketNames` (`self.Jetpack`))
          (if (`KismetStringLibrary.Contains` (`KismetStringLibrary.Conv_NameToString` _array_element_2) "Exhaust")
            (bind _returnvalue (`GameplayStatics.SpawnEmitterAttached` (`KismetArrayLibrary.Array_Get` (`self.Jetpack Exhaust Particles`) (`KismetMathLibrary.Conv_ByteToInt` (`self.Current Jetpack Type`))) (`self.Jetpack`) _array_element_2 (0.0 0.0 0.0) (struct) "SnapToTargetIncludingScale"))
            (`KismetArrayLibrary.Array_Add` (`self.Particles`) _returnvalue)
            (`ParticleSystemComponent.SetFloatParameter` _returnvalue "Scale" (select `bool` (`self.Jetpack_Flying`) :`true` 1.0 :!type "Float (single-precision)")))))
      (:`then_1`
        ;;[1 1 1] Adds audio to each jetpacks engine
        (for _array_element_3 _sounds :!label _label_6
          (`/Engine/EditorBlueprintResources/StandardMacros.IsValid` _array_element_3
            (:`Is Valid`
              (`ActorComponent.K2_DestroyComponent` _array_element_3))))
        (`KismetArrayLibrary.Array_Clear` _sounds)
        (for _array_element_4 (`SceneComponent.GetAllSocketNames` (`self.Jetpack`))
          (if (`KismetStringLibrary.Contains` (`KismetStringLibrary.Conv_NameToString` _array_element_4) (select `bool` (or (`|EnumEquality` _current_jetpack_type_2 "NewEnumerator2") (`|EnumEquality` "NewEnumerator6" _current_jetpack_type_2)) :`false` "Exhaust" :`true` "Audio_Source"))
            (bind _returnvalue_2 (`GameplayStatics.SpawnSoundAttached` (`KismetArrayLibrary.Array_Get` (`self.Jetpack Audio`) (`KismetMathLibrary.Conv_ByteToInt` (`self.Current Jetpack Type`))) (`self.Jetpack`) _array_element_4 (0.0 0.0 0.0) (struct) "SnapToTarget" true (+ (* (`KismetMathLibrary.Conv_BoolToDouble` (`self.Jetpack_Flying`)) 0.35) (/ (+ (`self.Forward`) (`self.Right`) (`self.Up`)) 6.0)) 1.0 (`KismetMathLibrary.RandomFloatInRange` 0.0 1.0)))
            (`KismetArrayLibrary.Array_Add` (`self.Sounds`) _returnvalue_2))))
      (:`then_2`
        ;;[1 1 1] Create dynamic materials for special visuals on winged/grav jetpacks
        (bind _returnvalue_3 (`PrimitiveComponent.CreateDynamicMaterialInstance` (`self.Jetpack`) 0 null))
        (set `self.Jetpack_MI` _returnvalue_3)
        (set `self.Jetpack Heat Level` 0.0)
        (if (`|EnumEquality` _current_jetpack_type "NewEnumerator6")
          (bind _returnvalue_4 (`PrimitiveComponent.CreateDynamicMaterialInstance` _jetpack_3 1 null))
          (set `self.Wings_MI` _returnvalue_4)
          (`MaterialInstanceDynamic.SetScalarParameterValue` (`self.Wings_MI`) "Opacity" (`KismetMathLibrary.Conv_BoolToDouble` (`self.Using Jetpack`)))
          (elif (`|EnumEquality` _current_jetpack_type "NewEnumerator2")
            (bind _returnvalue_5 (`PrimitiveComponent.CreateDynamicMaterialInstance` _jetpack_3 1 null))
            (set `self.Grav_MI` _returnvalue_5)))))))

(event `Rebuild Particles`
  ;[1 1 1] Update the type of jetpack/meshes used, and set up the required values/mesh location for it.
  ;;[1 1 1] Spawn exhausts
  (goto _label_5))

(event `Rebuild Audio`
  ;[1 1 1] Update the type of jetpack/meshes used, and set up the required values/mesh location for it.
  ;;[1 1 1] Adds audio to each jetpacks engine
  (goto _label_6))

(fn `Clear Particles`
  (bind _particles (`self.Particles`))
  ;[1 1 1] Clear all existing particles
  (for _array_element _particles
    (`/Engine/EditorBlueprintResources/StandardMacros.IsValid` _array_element
      (:`Is Valid`
        (`ActorComponent.K2_DestroyComponent` _array_element))))
  (`KismetArrayLibrary.Array_Clear` _particles)
  (return))

(fn `Update Audio Multiplier`
  (bind _current_jetpack_type (`self.Current Jetpack Type`))
  (bind _flying_audio_lerp (`self.Flying Audio Lerp`))
  (bind _returnvalue (`KismetMathLibrary.Conv_ByteToInt` (`self.Current Jetpack Type`)))
  (bind _returnvalue_2 (or (`|EnumEquality` _current_jetpack_type "NewEnumerator2") (`|EnumEquality` "NewEnumerator4" _current_jetpack_type)))
  (bind _returnvalue_3 (* (+ (* _flying_audio_lerp 0.35) (* _flying_audio_lerp (/ (+ (`KismetMathLibrary.Abs` (`self.Forward`)) (`KismetMathLibrary.Abs` (`self.Right`)) (`KismetMathLibrary.FClamp` (`self.Up`) -0.4)) 9.0) (`KismetMathLibrary.Conv_BoolToDouble` (`self.Jetpack_Flying`)))) (`KismetArrayLibrary.Array_Get` (`self.Jetpack Audio Multiplier`) _returnvalue)))
  ;[1 1 1] Adjust master multiplier for audio. Turns off sounds when engines are off, but over a short period and not an instant stop.
  (set `self.Flying Audio Lerp` (`KismetMathLibrary.FInterpTo` (`self.Flying Audio Lerp`) (select `bool` (`self.Jetpack_Flying`) :`false` (select `bool` (and _returnvalue_2 (`self.Using Jetpack`)) :`true` 0.35 :!type "Float (single-precision)") :`true` 1.0) (`GameplayStatics.GetWorldDeltaSeconds`) (`KismetMathLibrary.Lerp` 3.0 0.5 (`KismetMathLibrary.Conv_BoolToDouble` _returnvalue_2))))
  ;[1 1 1] Modify the volume based on input values (louder when flying up/moving/etc...
  (for _array_element (`self.Sounds`)
    (`/Engine/EditorBlueprintResources/StandardMacros.IsValid` _array_element
      (:`Is Valid`
        (`AudioComponent.SetVolumeMultiplier` _array_element _returnvalue_3)
        (`AudioComponent.SetPitchMultiplier` _array_element (* (`KismetMathLibrary.MapRangeClamped` _returnvalue_3 0.1 2.0 0.8 1.2) (`KismetArrayLibrary.Array_Get` (`self.Jetpack Pitch Multiplier`) _returnvalue)))))))

(fn `UserConstructionScript`
  (`self.Update Type`)
  (`SceneComponent.SetRelativeScale3D` (`self.Jetpack`) (`KismetMathLibrary.Conv_DoubleToVector` (`self.Jetpack Scale`))))