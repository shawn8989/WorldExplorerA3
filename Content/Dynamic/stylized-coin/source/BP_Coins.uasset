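; BP_Coins is a coin pickup that adds one point to the player's jetpack character when collected.
; Any overlap on its Trigger component casts player 0's character to BP_JetPackCharacter and increments that character's Score, without checking which actor overlapped.
; It then prints the score on screen, plays an attenuated coin sound, spawns a pickup Niagara effect and destroys itself.
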(event `self.ReceiveActorBeginOverlap`
  (params (OtherActor :type "Actor Object Reference")))

(event `self.Trigger.OnComponentBeginOverlap`
  (params (OverlappedComponent :type "PrimitiveComponent Object Reference") (OtherActor :type "Actor Object Reference") (OtherComp :type "PrimitiveComponent Object Reference") (OtherBodyIndex :type Integer) (bFromSweep :type Boolean) (SweepResult :type "HitResult Structure (by ref)"))
  (bind _returnvalue (`self.K2_GetActorLocation`))
  ;[0.4479 0.4479 0.4479] Increase the score being displalayed by 1 when collision occurs with coin
  (bind _asbp_jet_pack_character (cast `/Game/Dynamic/ThirdPerson/Blueprints/BP_JetPackCharacter` (`GameplayStatics.GetPlayerCharacter` 0)))
  (bind _output_get (set `/Game/Dynamic/ThirdPerson/Blueprints/BP_JetPackCharacter.Score` (+ 1 (`/Game/Dynamic/ThirdPerson/Blueprints/BP_JetPackCharacter.Score` _asbp_jet_pack_character)) _asbp_jet_pack_character))
  (`KismetSystemLibrary.PrintString` (`KismetStringLibrary.Conv_IntToString` _output_get) true true (struct :`R` 1.0 :`G` 0.17649 :`B` 0.206339 :`A` 1.0) 5.0)
  (`GameplayStatics.PlaySoundAtLocation` "/Game/341695__projectsu012__coins-1.341695__projectsu012__coins-1" _returnvalue (struct) 1.0 1.0 0.0 "/Game/SA_Coin.SA_Coin" null null null)
  (`NiagaraFunctionLibrary.SpawnSystemAtLocation` "/Game/Dynamic/stylized-coin/source/NS_CoinPickUp.NS_CoinPickUp" _returnvalue)
  (`self.K2_DestroyActor`))

(fn `UserConstructionScript`)