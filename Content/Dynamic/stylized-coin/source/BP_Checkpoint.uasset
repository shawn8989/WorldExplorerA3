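; BP_Checkpoint is a trigger-based checkpoint actor for the third-person game.
; When a BP_ThirdPersonCharacter overlaps its Trigger, it registers itself as LastCheckpoint on BP_ThirdPersonGameMode and plays a 2D explosion sound.
; It then adds zero to the player character's Score, leaving the value unchanged.
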(event `self.Trigger.OnComponentBeginOverlap`
  (params (OverlappedComponent :type "PrimitiveComponent Object Reference") (OtherActor :type "Actor Object Reference") (OtherComp :type "PrimitiveComponent Object Reference") (OtherBodyIndex :type Integer) (bFromSweep :type Boolean) (SweepResult :type "HitResult Structure (by ref)"))
  ;[1 1 1] Checkpoint for Third person
  (cast `/Game/Dynamic/ThirdPerson/Blueprints/BP_ThirdPersonCharacter` OtherActor)
  (bind _asbp_third_person_game_mode (cast `/Game/Dynamic/ThirdPerson/Blueprints/BP_ThirdPersonGameMode` (`GameplayStatics.GetGameMode`)))
  (set `/Game/Dynamic/ThirdPerson/Blueprints/BP_ThirdPersonGameMode.Last Checkpoint` self _asbp_third_person_game_mode)
  (`GameplayStatics.PlaySound2D` "/Game/StarterContent/Audio/Explosion01.Explosion01" 1.0 1.0 0.0 null null)
  (bind _asbp_third_person_character (cast `/Game/Dynamic/ThirdPerson/Blueprints/BP_ThirdPersonCharacter` (`GameplayStatics.GetPlayerCharacter` 0)))
  (set `/Game/Dynamic/ThirdPerson/Blueprints/BP_ThirdPersonCharacter.Score` (+ 0 (`/Game/Dynamic/ThirdPerson/Blueprints/BP_ThirdPersonCharacter.Score` _asbp_third_person_character)) _asbp_third_person_character))

(fn `UserConstructionScript`)