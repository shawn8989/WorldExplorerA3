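; BP_CoinsLarge is a coin pickup that adds one to the player's score.
; When its Trigger component is overlapped by a BP_ThirdPersonCharacter, it increments the Score stored on that character and prints the new total on screen.
; It then plays a coin sound, spawns the NS_CoinPickUp Niagara effect at its location and destroys itself.
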(event `self.ReceiveActorBeginOverlap`
  (params (OtherActor :type "Actor Object Reference"))
  ;[0.4479 0.4479 0.4479] Increase the score being displalayed by 1 when collision occurs with coin
)

(event `self.Trigger.OnComponentBeginOverlap`
  (params (OverlappedComponent :type "PrimitiveComponent Object Reference") (OtherActor :type "Actor Object Reference") (OtherComp :type "PrimitiveComponent Object Reference") (OtherBodyIndex :type Integer) (bFromSweep :type Boolean) (SweepResult :type "HitResult Structure (by ref)"))
  (bind _returnvalue (`self.K2_GetActorLocation`))
  ;[0.4479 0.4479 0.4479] Increase the score being displalayed by 1 when collision occurs with coin
  (bind _asbp_third_person_character (cast `/Game/Dynamic/ThirdPerson/Blueprints/BP_ThirdPersonCharacter` OtherActor))
  (set `/Game/Dynamic/ThirdPerson/Blueprints/BP_ThirdPersonCharacter.Score` (+ (`/Game/Dynamic/ThirdPerson/Blueprints/BP_ThirdPersonCharacter.Score` _asbp_third_person_character) 1) _asbp_third_person_character)
  (`KismetSystemLibrary.PrintString` (`KismetStringLibrary.Conv_IntToString` (`/Game/Dynamic/ThirdPerson/Blueprints/BP_ThirdPersonCharacter.Score` _asbp_third_person_character)) true true (struct :`R` 1.0 :`G` 0.17649 :`B` 0.206339 :`A` 1.0) 5.0)
  (`GameplayStatics.PlaySoundAtLocation` "/Game/341695__projectsu012__coins-1.341695__projectsu012__coins-1" _returnvalue (struct) 1.0 1.0 0.0 null null null null)
  (`NiagaraFunctionLibrary.SpawnSystemAtLocation` "/Game/Dynamic/stylized-coin/source/NS_CoinPickUp.NS_CoinPickUp" _returnvalue)
  (`self.K2_DestroyActor`))

(fn `UserConstructionScript`)